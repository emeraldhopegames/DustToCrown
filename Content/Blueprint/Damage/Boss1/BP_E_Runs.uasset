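; BP_E_Runs is a sprite-based character hazard, filed under Boss1 damage, that launches itself on spawn and hurts the hero on contact.
; BeginPlay randomly picks positive or negative X and launches the character using a suggested arc velocity between fixed offsets.
; A Box overlap applies damage to BP_Hero.
; A SpawnDust function, not called in this graph, spawns BP_LandDust at the sprite's location and rotation.
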(event `self.ReceiveBeginPlay`
  (switch `int` (`KismetMathLibrary.RandomIntegerInRange` 0 1)
    (:`0`
      (bind _outlaunchvelocity (`GameplayStatics.SuggestProjectileVelocity_CustomArc` (0.0 0.0 0.0) (100.0 0.0 0.0)))
      (`self.LaunchCharacter` _outlaunchvelocity))
    (:`1`
      (bind _outlaunchvelocity_2 (`GameplayStatics.SuggestProjectileVelocity_CustomArc` (0.0 0.0 0.0) (-100.0 0.0 0.0)))
      (`self.LaunchCharacter` _outlaunchvelocity_2))))

(event `self.Box.OnComponentBeginOverlap`
  (params (OverlappedComponent :type "PrimitiveComponent Object Reference") (OtherActor :type "Actor Object Reference") (OtherComp :type "PrimitiveComponent Object Reference") (OtherBodyIndex :type Integer) (bFromSweep :type Boolean) (SweepResult :type "HitResult Structure (by ref)"))
  (bind _asbp_hero (cast `/Game/Blueprint/Hero/BP_Hero` OtherActor))
  (`GameplayStatics.ApplyDamage` _asbp_hero 1.0))

(fn `SpawnDust`
  (bind (_returnvalue_location _returnvalue_rotation) (`KismetMathLibrary.BreakTransform` (`SceneComponent.K2_GetComponentToWorld` (`self.Sprite`))))
  (`|SpawnActorFromClass` "/Game/Blueprint/Hero/BP_LandDust.BP_LandDust_C" (`KismetMathLibrary.MakeTransform` _returnvalue_location _returnvalue_rotation) "Undefined" "MultiplyWithRoot" null null))

(fn `UserConstructionScript`)