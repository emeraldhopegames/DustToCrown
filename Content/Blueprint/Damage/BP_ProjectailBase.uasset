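; Base projectile Blueprint that damages the hero or turns into an enemy when it hits a stopper.
; The construction script applies the Speed and Gravity variables to the projectile movement component.
; On box overlap it damages a BP_Hero that is not rolling, then destroys itself, so rolling heroes avoid it.
; Overlapping a BP_Stop spawns a BP_E_Runs AI pawn near its location and destroys the projectile.
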(event `self.Box.OnComponentBeginOverlap`
  (params (OverlappedComponent :type "PrimitiveComponent Object Reference") (OtherActor :type "Actor Object Reference") (OtherComp :type "PrimitiveComponent Object Reference") (OtherBodyIndex :type Integer) (bFromSweep :type Boolean) (SweepResult :type "HitResult Structure (by ref)"))
  (bind (_returnvalue_x _returnvalue_y _returnvalue_z) (`KismetMathLibrary.BreakVector` (`self.K2_GetActorLocation`)))
  (`|ExecutionSequence`
    (:`then_0`
      (bind _asbp_hero (cast `/Game/Blueprint/Hero/BP_Hero` OtherActor))
      (if (not (`/Game/Blueprint/Hero/BP_Hero.Roll` _asbp_hero))
        (`GameplayStatics.ApplyDamage` _asbp_hero 1.0)
        (`self.K2_DestroyActor`)))
    (:`then_1`
      (cast `/Game/Blueprint/Damage/BP_Stop` OtherActor)
      (`AIBlueprintHelperLibrary.SpawnAIFromClass` "/Game/Blueprint/Damage/Boss1/BP_E_Runs.BP_E_Runs_C" null (`KismetMathLibrary.MakeVector` _returnvalue_x (- _returnvalue_y 2.0) _returnvalue_z) (struct) false null)
      (`self.K2_DestroyActor`))))

(fn `UserConstructionScript`
  (bind _projectilemovement (`self.ProjectileMovement`))
  (bind _speed (`self.Speed`))
  (set `ProjectileMovementComponent.InitialSpeed` _speed _projectilemovement)
  (set `ProjectileMovementComponent.MaxSpeed` _speed _projectilemovement)
  (set `ProjectileMovementComponent.ProjectileGravityScale` (`self.Gravity`) _projectilemovement))