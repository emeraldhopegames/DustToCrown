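; Main game mode that spawns and possesses each player's chosen character, BP_Light or BP_Shadow, when play begins.
; One tick after BeginPlay, it reads the two-player flag and character picks from the first controller's PC_Main.
; In two-player mode it creates a second local player and places both characters at the first two PlayerStarts found.
; Otherwise it spawns only the selected character at the first start.
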(event `self.ReceiveBeginPlay`
  (`KismetSystemLibrary.DelayUntilNextTick`)
  (bind _outactors (`GameplayStatics.GetAllActorsOfClass` "/Script/Engine.PlayerStart"))
  (bind _aspc_main (cast `/Game/Blueprint/GM/PC_Main` (`GameplayStatics.GetPlayerController` 0)))
  (if (`/Game/Blueprint/GM/PC_Main.2Player?` _aspc_main)
    (for _index (range 2)
      (if (> _index 0)
        (`GameplayStatics.CreatePlayer` -1)
        (switch `int` (`/Game/Blueprint/GM/PC_Main.2PlayerChar` _aspc_main)
          (:`0`
            (bind _returnvalue (`self.GetTransform` (`|GetArrayItem` _outactors 1)))
            (bind _returnvalue_2 (`|SpawnActorFromClass` "/Game/Blueprint/Hero/BP_Light.BP_Light_C" _returnvalue "Undefined" "MultiplyWithRoot" null 0 null))
            (`Controller.Possess` (`GameplayStatics.GetPlayerController` 1) _returnvalue_2))
          (:`1`
            (bind _returnvalue_3 (`|SpawnActorFromClass` "/Game/Blueprint/Hero/BP_Shadow.BP_Shadow_C" _returnvalue "Undefined" "MultiplyWithRoot" null null))
            (`Controller.Possess` (`GameplayStatics.GetPlayerController` 1) _returnvalue_3)))
        (else
          (switch `int` (`/Game/Blueprint/GM/PC_Main.1PlayerChar` _aspc_main)
            (:`0`
              (bind _returnvalue_4 (`self.GetTransform` (`|GetArrayItem` _outactors)))
              (bind _returnvalue_5 (`|SpawnActorFromClass` "/Game/Blueprint/Hero/BP_Light.BP_Light_C" _returnvalue_4 "Undefined" "MultiplyWithRoot" null 0 null))
              (`Controller.Possess` (`GameplayStatics.GetPlayerController` 0) _returnvalue_5))
            (:`1`
              (bind _returnvalue_6 (`|SpawnActorFromClass` "/Game/Blueprint/Hero/BP_Shadow.BP_Shadow_C" _returnvalue_4 "Undefined" "MultiplyWithRoot" null null))
              (`Controller.Possess` (`GameplayStatics.GetPlayerController` 0) _returnvalue_6))))))
    (else
      (switch `int` (`/Game/Blueprint/GM/PC_Main.SelectChar` _aspc_main)
        (:`0`
          (bind _returnvalue_7 (`|SpawnActorFromClass` "/Game/Blueprint/Hero/BP_Light.BP_Light_C" _returnvalue_4 "Undefined" "MultiplyWithRoot" null 0 null))
          (`Controller.Possess` (`GameplayStatics.GetPlayerController` 0) _returnvalue_7))
        (:`1`
          (bind _returnvalue_8 (`|SpawnActorFromClass` "/Game/Blueprint/Hero/BP_Shadow.BP_Shadow_C" _returnvalue_4 "Undefined" "MultiplyWithRoot" null null))
          (`Controller.Possess` (`GameplayStatics.GetPlayerController` 0) _returnvalue_8))))))

(fn `UserConstructionScript`)