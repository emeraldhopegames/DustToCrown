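; Main player controller that saves and loads the two-player flag and character selection state for both players.
; SaveBool copies these variables into a new BP_SaveBool object and writes it to the "Bool" slot.
; BeginPlay calls LoadBool, which restores them from that slot if the cast succeeds.
; A delayed IMC_Main Enhanced Input mapping setup is present but never runs.
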(event `self.ReceiveBeginPlay`
  (`self.LoadBool`))

(event `SaveBool`
  ; SaveLoad
  (bind _returnvalue (`GameplayStatics.CreateSaveGameObject` "/Game/Blueprint/Save/BP_SaveBool.BP_SaveBool_C"))
  (bind _output_get (set `self.SaveB` _returnvalue))
  (set `/Game/Blueprint/Save/BP_SaveBool.2Player?` (`self.2Player?`) _output_get)
  (set `/Game/Blueprint/Save/BP_SaveBool.SelectChar` (`self.SelectChar`) _returnvalue)
  (set `/Game/Blueprint/Save/BP_SaveBool.1PlayerChar` (`self.1PlayerChar`) _returnvalue)
  (set `/Game/Blueprint/Save/BP_SaveBool.2PlayerChar` (`self.2PlayerChar`) _returnvalue)
  (`GameplayStatics.SaveGameToSlot` _output_get "Bool"))

(event `LoadBool`
  ; SaveLoad
  (bind _returnvalue (`GameplayStatics.LoadGameFromSlot` "Bool"))
  (bind _asbp_save_bool (cast `/Game/Blueprint/Save/BP_SaveBool` _returnvalue))
  (bind _output_get (set `self.SaveB` _asbp_save_bool))
  (set `self.2Player?` (`/Game/Blueprint/Save/BP_SaveBool.2Player?` _output_get))
  (set `self.SelectChar` (`/Game/Blueprint/Save/BP_SaveBool.SelectChar` _output_get))
  (set `self.1PlayerChar` (`/Game/Blueprint/Save/BP_SaveBool.1PlayerChar` _output_get))
  (set `self.2PlayerChar` (`/Game/Blueprint/Save/BP_SaveBool.2PlayerChar` _output_get)))

(fn `UserConstructionScript`)