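; BP_DoorToBoss is a door that opens another level when interacted with, by its name a passage to a boss.
; Its Box collision creates and shows a WBP_DoorName widget when a BP_Light actor enters, and removes it when that actor leaves.
; The Interact event loads the level named by the LevelName variable, with no overlap check of its own.
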(event `self.Box.OnComponentBeginOverlap`
  (params (OverlappedComponent :type "PrimitiveComponent Object Reference") (OtherActor :type "Actor Object Reference") (OtherComp :type "PrimitiveComponent Object Reference") (OtherBodyIndex :type Integer) (bFromSweep :type Boolean) (SweepResult :type "HitResult Structure (by ref)"))
  (cast `/Game/Blueprint/Hero/BP_Light` OtherActor)
  (bind _returnvalue (`|CreateWidget` "/Game/Blueprint/Widget/WBP_DoorName.WBP_DoorName_C"))
  (bind _output_get (set `self.Widget` _returnvalue))
  (`UserWidget.AddToViewport` _output_get 0))

(event `self.Box.OnComponentEndOverlap`
  (params (OverlappedComponent :type "PrimitiveComponent Object Reference") (OtherActor :type "Actor Object Reference") (OtherComp :type "PrimitiveComponent Object Reference") (OtherBodyIndex :type Integer))
  (cast `/Game/Blueprint/Hero/BP_Light` OtherActor)
  (`Widget.RemoveFromParent` (`self.Widget`)))

(event `/Game/Blueprint/BPI_Interact.Interact`
  (`GameplayStatics.OpenLevel` (`self.Level Name`)))

(fn `UserConstructionScript`)