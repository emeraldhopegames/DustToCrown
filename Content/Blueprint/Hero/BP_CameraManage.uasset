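; BP_CameraManage is a shared camera actor that frames two BP_MainChar characters at once.
; When GM_Main triggers its camera setup event, it becomes player 0's view target and caches all BP_MainChar actors.
; Each Tick moves it to the midpoint of the first two characters and sets spring arm length from their clamped separation, zooming out as they spread apart.
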(event `self.ReceiveBeginPlay`
  (bind _asgm_main (cast `/Game/Blueprint/GM/GM_Main` (`GameplayStatics.GetGameMode`)))
  (add `/Game/Blueprint/GM/GM_Main.SetupCamera` _asgm_main (delegate `Init`)))

(event `Init`
  (`PlayerController.SetViewTargetWithBlend` (`GameplayStatics.GetPlayerController` 0) self 0.0 "VTBlend_Linear" 0.0 false)
  (bind _outactors (`GameplayStatics.GetAllActorsOfClass` "/Game/Blueprint/Hero/Character/BP_MainChar.BP_MainChar_C"))
  (set `self.Characters` _outactors))

(event `self.ReceiveTick`
  (params (DeltaSeconds :type "Float (single-precision)"))
  (bind _characters (`self.Characters`))
  (bind _output (`|GetArrayItem` _characters))
  (bind _output_2 (`|GetArrayItem` _characters 1))
  (set `SpringArmComponent.TargetArmLength` (`KismetMathLibrary.FClamp` (* (`self.GetDistanceTo` _output _output_2) 1.0) 500.0 2500.0) (`self.SpringArm`))
  (`self.K2_SetActorLocation` (`KismetMathLibrary.VLerp` (`self.K2_GetActorLocation` _output) (`self.K2_GetActorLocation` _output_2) 0.5)))

(fn `UserConstructionScript`)