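; AN_Attack is an animation notify for hero attacks that applies a fixed amount of damage to pawns inside a box.
; With a valid owning instance, it box-overlaps at the sequence render component's location, ignoring the owner and the first two player characters, then damages and prints each hit.
; Without an instance, it draws a green debug box of the same extent instead.
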(fn `OnReceiveNotify`
  (params (OwningInstance :type "PaperZDAnimInstance Object Reference"))
  (bind _extent (`self.Extent`))
  (bind _returnvalue (`SceneComponent.K2_GetComponentLocation` (`self.SequenceRenderComponent`)))
  (`/Engine/EditorBlueprintResources/StandardMacros.IsValid` OwningInstance
    (:`Is Valid`
      (bind _outactors (`KismetSystemLibrary.BoxOverlapActors` _returnvalue _extent (`|MakeArray` "ObjectTypeQuery3" :!type "EObjectTypeQuery Enum") null (`|MakeArray` (`PaperZDAnimInstance.GetOwningActor` OwningInstance) (`GameplayStatics.GetPlayerCharacter` 0) (`GameplayStatics.GetPlayerCharacter` 1) :!type "Actor Object Reference")))
      (for _array_element _outactors
        (`KismetSystemLibrary.PrintString` (`KismetSystemLibrary.GetDisplayName` _array_element))
        (`GameplayStatics.ApplyDamage` _array_element 10.0))
      (`KismetSystemLibrary.PrintString` "No more"))
    (:`Is Not Valid`
      (`KismetSystemLibrary.DrawDebugBox` _returnvalue _extent (struct :`R` 0.197969 :`G` 1.0 :`A` 1.0)))))