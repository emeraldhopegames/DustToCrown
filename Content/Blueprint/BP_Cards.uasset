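; BP_Cards is an interactable card actor that opens a card UI when used by the player.
; On Interact, it casts the player character to BP_Light and sets its walk speed to zero, then plays a sound and hides its static mesh.
; After a short delay, it creates WBP_Card and adds it to the viewport; walk speed is not restored here.
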(event `/Game/Blueprint/BPI_Interact.Interact`
  (bind _asbp_light (cast `/Game/Blueprint/Hero/Character/BP_Light` (`GameplayStatics.GetPlayerCharacter` 0)))
  (set `CharacterMovementComponent.MaxWalkSpeed` 0.0 (`Character.CharacterMovement` _asbp_light))
  (`GameplayStatics.PlaySoundAtLocation` (`self.Sound`) (`self.K2_GetActorLocation`) (struct) 1.0 1.0 0.0 null null null null)
  (`SceneComponent.SetVisibility` (`self.StaticMesh`) false false)
  (`KismetSystemLibrary.Delay` 0.3)
  (bind _returnvalue (`|CreateWidget` "/Game/Blueprint/Widget/WBP_Card.WBP_Card_C"))
  (`UserWidget.AddToViewport` _returnvalue 0))

(fn `UserConstructionScript`)