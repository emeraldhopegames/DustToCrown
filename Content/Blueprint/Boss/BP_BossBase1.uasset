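; BP_BossBase1 is a sprite-based boss actor that tracks health and deals contact damage.
; On BeginPlay it spawns a BP_ProjectailBase projectile at its own transform, passing a speed and a Niagara hit effect.
; Incoming damage is subtracted from Health with no death check, and anything overlapping its Box takes damage.
; A SpawnDust function places BP_LandDust at the sprite's location and rotation, but nothing here calls it.
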(event `self.ReceiveBeginPlay`
  (`|SpawnActorFromClass` "/Game/Blueprint/Damage/BP_ProjectailBase.BP_ProjectailBase_C" (`self.GetTransform`) "Undefined" "MultiplyWithRoot" null 1000.0 0.0 "/Game/sA_Megapack_v1/sA_Projectilevfx/Vfx/Fx/Niagara_Systems/NS_Hit7.NS_Hit7" null null))

(event `self.ReceiveAnyDamage`
  (params (Damage :type "Float (single-precision)") (DamageType :type "DamageType Object Reference") (InstigatedBy :type "Controller Object Reference") (DamageCauser :type "Actor Object Reference"))
  (set `self.Health` (- (`self.Health`) Damage)))

(event `self.Box.OnComponentBeginOverlap`
  (params (OverlappedComponent :type "PrimitiveComponent Object Reference") (OtherActor :type "Actor Object Reference") (OtherComp :type "PrimitiveComponent Object Reference") (OtherBodyIndex :type Integer) (bFromSweep :type Boolean) (SweepResult :type "HitResult Structure (by ref)"))
  (`GameplayStatics.ApplyDamage` OtherActor 1.0))

(fn `SpawnDust`
  (bind (_returnvalue_location _returnvalue_rotation) (`KismetMathLibrary.BreakTransform` (`SceneComponent.K2_GetComponentToWorld` (`self.Sprite`))))
  (`|SpawnActorFromClass` "/Game/Blueprint/Hero/BP_LandDust.BP_LandDust_C" (`KismetMathLibrary.MakeTransform` _returnvalue_location _returnvalue_rotation) "Undefined" "MultiplyWithRoot" null null))

(fn `UserConstructionScript`)