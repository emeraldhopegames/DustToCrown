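; Slime boss character that runs a self-repeating random attack loop from BeginPlay, with its attack pool changing at two health thresholds.
; Attacks include arced leaps between fixed points, a full-area hazard, timed projectile waves and a single BP_ProjectailLyc shot, paired in the lowest-health phase.
; Damage triggers Hurt or Dead animation jumps, and death spawns BP_Cards.
; An overlap box deals contact damage to BP_Hero, throttled by a Delay on Tick.
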(event `Attack5`
  (bind _returnvalue (`self.GetTransform`))
  ;[0.15 0.15 0.15 0.5 100] Attack5
  (set `self.Attack5?` true)
  (`GameplayStatics.PlaySound2D` null 1.0 1.0 0.0 null null)
  (`KismetSystemLibrary.Delay` 1.0)
  (`|SpawnActorFromClass` "/Game/Blueprint/Damage/BP_ProjectailLyc.BP_ProjectailLyc_C" (`KismetMathLibrary.MakeTransform` (`KismetMathLibrary.MakeVector` (- (.x (.location _returnvalue)) 100.0) (.y (.location _returnvalue)) (- (.z (.location _returnvalue)) 100.0)) (.rotation _returnvalue) (1.2 0.5 0.5)) "Undefined" "MultiplyWithRoot" null "/Game/sA_Megapack_v1/sA_Projectilevfx/Vfx/Fx/Niagara_Systems/NS_Hit7.NS_Hit7" null null)
  (set `self.Attack5?` false))

(event `Attack4`
  (bind _returnvalue (`self.GetTransform`))
  (bind _returnvalue_2 (`self.GetTransform`))
  (bind _returnvalue_3 (`self.GetTransform`))
  (bind _returnvalue_4 (`self.GetTransform`))
  (bind _returnvalue_5 (`self.GetTransform`))
  (bind _returnvalue_6 (`self.GetTransform`))
  (bind _returnvalue_7 (`self.GetTransform`))
  (bind _returnvalue_8 (`self.GetTransform`))
  (bind _returnvalue_9 (`self.GetTransform`))
  (bind _returnvalue_10 (`self.GetTransform`))
  (bind _returnvalue_11 (`self.GetTransform`))
  (bind _returnvalue_12 (`self.GetTransform`))
  ;[0.15 0.15 0.15 0.5 100] Attack4
  ;;[0.01207 0.15 0 0.5 100] Fist Wave
  (`GameplayStatics.PlaySound2D` null 1.0 1.0 0.0 null null)
  (`KismetSystemLibrary.Delay` 0.2)
  (set `self.Attack4?` true)
  (`|SpawnActorFromClass` "/Game/Blueprint/Damage/BP_ProjectailBase.BP_ProjectailBase_C" (`KismetMathLibrary.MakeTransform` (`KismetMathLibrary.MakeVector` (- (.x (.location _returnvalue_11)) 1500.0) (.y (.location _returnvalue_11)) (+ (.z (.location _returnvalue_11)) 600.0)) (.rotation _returnvalue_11) (.scale _returnvalue_11)) "Undefined" "MultiplyWithRoot" null 0.0 1.0 "/Game/sA_Megapack_v1/sA_Projectilevfx/Vfx/Fx/Niagara_Systems/NS_Hit7.NS_Hit7" null null)
  (`KismetSystemLibrary.Delay` 0.5)
  (`|SpawnActorFromClass` "/Game/Blueprint/Damage/BP_ProjectailBase.BP_ProjectailBase_C" (`KismetMathLibrary.MakeTransform` (`KismetMathLibrary.MakeVector` (- (.x (.location _returnvalue_5)) 1000.0) (.y (.location _returnvalue_5)) (+ (.z (.location _returnvalue_5)) 600.0)) (.rotation _returnvalue_5) (.scale _returnvalue_5)) "Undefined" "MultiplyWithRoot" null 0.0 0.5 "/Game/sA_Megapack_v1/sA_Projectilevfx/Vfx/Fx/Niagara_Systems/NS_Hit7.NS_Hit7" null null)
  (`KismetSystemLibrary.Delay` 0.5)
  (`|SpawnActorFromClass` "/Game/Blueprint/Damage/BP_ProjectailBase.BP_ProjectailBase_C" (`KismetMathLibrary.MakeTransform` (`KismetMathLibrary.MakeVector` (- (.x (.location _returnvalue_3)) 500.0) (.y (.location _returnvalue_3)) (+ (.z (.location _returnvalue_3)) 600.0)) (.rotation _returnvalue_3) (.scale _returnvalue_3)) "Undefined" "MultiplyWithRoot" null 0.0 0.8 "/Game/sA_Megapack_v1/sA_Projectilevfx/Vfx/Fx/Niagara_Systems/NS_Hit7.NS_Hit7" null null)
  (`KismetSystemLibrary.Delay` 0.5)
  (`|SpawnActorFromClass` "/Game/Blueprint/Damage/BP_ProjectailBase.BP_ProjectailBase_C" (`KismetMathLibrary.MakeTransform` (`KismetMathLibrary.MakeVector` (- (.x (.location _returnvalue_6)) 0.0) (.y (.location _returnvalue_6)) (+ (.z (.location _returnvalue_6)) 600.0)) (.rotation _returnvalue_6) (.scale _returnvalue_6)) "Undefined" "MultiplyWithRoot" null 0.0 0.9 "/Game/sA_Megapack_v1/sA_Projectilevfx/Vfx/Fx/Niagara_Systems/NS_Hit7.NS_Hit7" null null)
  ;;[0.15 0.002187 0 0.5 100] Two Wave
  (`KismetSystemLibrary.Delay` 1.0)
  (`|SpawnActorFromClass` "/Game/Blueprint/Damage/BP_ProjectailBase.BP_ProjectailBase_C" (`KismetMathLibrary.MakeTransform` (`KismetMathLibrary.MakeVector` (- (.x (.location _returnvalue_7)) 1250.0) (.y (.location _returnvalue_7)) (+ (.z (.location _returnvalue_7)) 600.0)) (.rotation _returnvalue_7) (.scale _returnvalue_7)) "Undefined" "MultiplyWithRoot" null 0.7 0.7 "/Game/sA_Megapack_v1/sA_Projectilevfx/Vfx/Fx/Niagara_Systems/NS_Hit7.NS_Hit7" null null)
  (`KismetSystemLibrary.Delay` 0.5)
  (`|SpawnActorFromClass` "/Game/Blueprint/Damage/BP_ProjectailBase.BP_ProjectailBase_C" (`KismetMathLibrary.MakeTransform` (`KismetMathLibrary.MakeVector` (- (.x (.location _returnvalue_8)) 750.0) (.y (.location _returnvalue_8)) (+ (.z (.location _returnvalue_8)) 600.0)) (.rotation _returnvalue_8) (.scale _returnvalue_8)) "Undefined" "MultiplyWithRoot" null 0.0 0.5 "/Game/sA_Megapack_v1/sA_Projectilevfx/Vfx/Fx/Niagara_Systems/NS_Hit7.NS_Hit7" null null)
  (`KismetSystemLibrary.Delay` 0.5)
  (`|SpawnActorFromClass` "/Game/Blueprint/Damage/BP_ProjectailBase.BP_ProjectailBase_C" (`KismetMathLibrary.MakeTransform` (`KismetMathLibrary.MakeVector` (- (.x (.location _returnvalue_4)) 250.0) (.y (.location _returnvalue_4)) (+ (.z (.location _returnvalue_4)) 600.0)) (.rotation _returnvalue_4) (.scale _returnvalue_4)) "Undefined" "MultiplyWithRoot" null 0.0 0.8 "/Game/sA_Megapack_v1/sA_Projectilevfx/Vfx/Fx/Niagara_Systems/NS_Hit7.NS_Hit7" null null)
  (`KismetSystemLibrary.Delay` 0.5)
  (`|SpawnActorFromClass` "/Game/Blueprint/Damage/BP_ProjectailBase.BP_ProjectailBase_C" (`KismetMathLibrary.MakeTransform` (`KismetMathLibrary.MakeVector` (+ (.x (.location _returnvalue_9)) 200.0) (.y (.location _returnvalue_9)) (+ (.z (.location _returnvalue_9)) 600.0)) (.rotation _returnvalue_9) (.scale _returnvalue_9)) "Undefined" "MultiplyWithRoot" null 0.0 1.0 "/Game/sA_Megapack_v1/sA_Projectilevfx/Vfx/Fx/Niagara_Systems/NS_Hit7.NS_Hit7" null null)
  ;;[0 0.01236 0.15 0.5 100] There WAVE
  (`KismetSystemLibrary.Delay` 1.0)
  (`|SpawnActorFromClass` "/Game/Blueprint/Damage/BP_ProjectailBase.BP_ProjectailBase_C" (`KismetMathLibrary.MakeTransform` (`KismetMathLibrary.MakeVector` (- (.x (.location _returnvalue_12)) 1600.0) (.y (.location _returnvalue_12)) (+ (.z (.location _returnvalue_12)) 600.0)) (.rotation _returnvalue_12) (.scale _returnvalue_12)) "Undefined" "MultiplyWithRoot" null 0.0 1.1 "/Game/sA_Megapack_v1/sA_Projectilevfx/Vfx/Fx/Niagara_Systems/NS_Hit7.NS_Hit7" null null)
  (`KismetSystemLibrary.Delay` 0.5)
  (`|SpawnActorFromClass` "/Game/Blueprint/Damage/BP_ProjectailBase.BP_ProjectailBase_C" (`KismetMathLibrary.MakeTransform` (`KismetMathLibrary.MakeVector` (- (.x (.location _returnvalue_2)) 1100.0) (.y (.location _returnvalue_2)) (+ (.z (.location _returnvalue_2)) 600.0)) (.rotation _returnvalue_2) (.scale _returnvalue_2)) "Undefined" "MultiplyWithRoot" null 0.0 0.7 "/Game/sA_Megapack_v1/sA_Projectilevfx/Vfx/Fx/Niagara_Systems/NS_Hit7.NS_Hit7" null null)
  (`KismetSystemLibrary.Delay` 0.5)
  (`|SpawnActorFromClass` "/Game/Blueprint/Damage/BP_ProjectailBase.BP_ProjectailBase_C" (`KismetMathLibrary.MakeTransform` (`KismetMathLibrary.MakeVector` (- (.x (.location _returnvalue_10)) 800.0) (.y (.location _returnvalue_10)) (+ (.z (.location _returnvalue_10)) 600.0)) (.rotation _returnvalue_10) (.scale _returnvalue_10)) "Undefined" "MultiplyWithRoot" null 0.0 0.8 "/Game/sA_Megapack_v1/sA_Projectilevfx/Vfx/Fx/Niagara_Systems/NS_Hit7.NS_Hit7" null null)
  (`KismetSystemLibrary.Delay` 0.5)
  (`|SpawnActorFromClass` "/Game/Blueprint/Damage/BP_ProjectailBase.BP_ProjectailBase_C" (`KismetMathLibrary.MakeTransform` (`KismetMathLibrary.MakeVector` (- (.x (.location _returnvalue)) 300.0) (.y (.location _returnvalue)) (+ (.z (.location _returnvalue)) 600.0)) (.rotation _returnvalue) (.scale _returnvalue)) "Undefined" "MultiplyWithRoot" null 0.0 0.6 "/Game/sA_Megapack_v1/sA_Projectilevfx/Vfx/Fx/Niagara_Systems/NS_Hit7.NS_Hit7" null null)
  (set `self.Attack4?` false))

(event `Attack3`
  (bind _returnvalue (`self.GetTransform`))
  (bind _returnvalue_2 (`self.GetTransform`))
  (bind _returnvalue_3 (`self.GetTransform`))
  (bind _returnvalue_4 (`self.GetTransform`))
  (bind _returnvalue_5 (`self.GetTransform`))
  (bind _returnvalue_6 (`self.GetTransform`))
  (bind _returnvalue_7 (`self.GetTransform`))
  (bind _returnvalue_8 (`self.GetTransform`))
  (bind _returnvalue_9 (`self.GetTransform`))
  ;[0.15 0.15 0.15 0.5 100] Attack3
  ;;[0.01207 0.15 0 0.5 100] Fist Wave
  (`GameplayStatics.PlaySound2D` null 1.0 1.0 0.0 null null)
  (`KismetSystemLibrary.Delay` 0.2)
  (set `self.Attack3?` true)
  (`|SpawnActorFromClass` "/Game/Blueprint/Damage/BP_ProjectailBase.BP_ProjectailBase_C" (`KismetMathLibrary.MakeTransform` (`KismetMathLibrary.MakeVector` (.x (.location _returnvalue)) (.y (.location _returnvalue)) (- (.z (.location _returnvalue)) 200.0)) (.rotation _returnvalue) (.scale _returnvalue)) "Undefined" "MultiplyWithRoot" null 600.0 0.0 "/Game/sA_Megapack_v1/sA_Projectilevfx/Vfx/Fx/Niagara_Systems/NS_Hit7.NS_Hit7" null null)
  (`KismetSystemLibrary.Delay` 0.5)
  (`|SpawnActorFromClass` "/Game/Blueprint/Damage/BP_ProjectailBase.BP_ProjectailBase_C" (`KismetMathLibrary.MakeTransform` (`KismetMathLibrary.MakeVector` (.x (.location _returnvalue_2)) (.y (.location _returnvalue_2)) (- (.z (.location _returnvalue_2)) 50.0)) (.rotation _returnvalue_2) (.scale _returnvalue_2)) "Undefined" "MultiplyWithRoot" null 400.0 0.0 "/Game/sA_Megapack_v1/sA_Projectilevfx/Vfx/Fx/Niagara_Systems/NS_Hit7.NS_Hit7" null null)
  (`KismetSystemLibrary.Delay` 0.5)
  (`|SpawnActorFromClass` "/Game/Blueprint/Damage/BP_ProjectailBase.BP_ProjectailBase_C" (`KismetMathLibrary.MakeTransform` (`KismetMathLibrary.MakeVector` (.x (.location _returnvalue_3)) (.y (.location _returnvalue_3)) (+ (.z (.location _returnvalue_3)) 50.0)) (.rotation _returnvalue_3) (.scale _returnvalue_3)) "Undefined" "MultiplyWithRoot" null 500.0 0.0 "/Game/sA_Megapack_v1/sA_Projectilevfx/Vfx/Fx/Niagara_Systems/NS_Hit7.NS_Hit7" null null)
  ;;[0.15 0.002187 0 0.5 100] Two Wave
  (`KismetSystemLibrary.Delay` 1.0)
  (`|SpawnActorFromClass` "/Game/Blueprint/Damage/BP_ProjectailBase.BP_ProjectailBase_C" (`KismetMathLibrary.MakeTransform` (`KismetMathLibrary.MakeVector` (.x (.location _returnvalue_4)) (.y (.location _returnvalue_4)) (- (.z (.location _returnvalue_4)) 200.0)) (.rotation _returnvalue_4) (.scale _returnvalue_4)) "Undefined" "MultiplyWithRoot" null 1000.0 0.0 "/Game/sA_Megapack_v1/sA_Projectilevfx/Vfx/Fx/Niagara_Systems/NS_Hit7.NS_Hit7" null null)
  (`KismetSystemLibrary.Delay` 0.5)
  (`|SpawnActorFromClass` "/Game/Blueprint/Damage/BP_ProjectailBase.BP_ProjectailBase_C" (`KismetMathLibrary.MakeTransform` (`KismetMathLibrary.MakeVector` (.x (.location _returnvalue_5)) (.y (.location _returnvalue_5)) (- (.z (.location _returnvalue_5)) 50.0)) (.rotation _returnvalue_5) (.scale _returnvalue_5)) "Undefined" "MultiplyWithRoot" null 600.0 0.0 "/Game/sA_Megapack_v1/sA_Projectilevfx/Vfx/Fx/Niagara_Systems/NS_Hit7.NS_Hit7" null null)
  (`KismetSystemLibrary.Delay` 0.5)
  (`|SpawnActorFromClass` "/Game/Blueprint/Damage/BP_ProjectailBase.BP_ProjectailBase_C" (`KismetMathLibrary.MakeTransform` (`KismetMathLibrary.MakeVector` (.x (.location _returnvalue_6)) (.y (.location _returnvalue_6)) (+ (.z (.location _returnvalue_6)) 50.0)) (.rotation _returnvalue_6) (.scale _returnvalue_6)) "Undefined" "MultiplyWithRoot" null 500.0 0.0 "/Game/sA_Megapack_v1/sA_Projectilevfx/Vfx/Fx/Niagara_Systems/NS_Hit7.NS_Hit7" null null)
  ;;[0 0.01236 0.15 0.5 100] There WAVE
  (`KismetSystemLibrary.Delay` 1.0)
  (`|SpawnActorFromClass` "/Game/Blueprint/Damage/BP_ProjectailBase.BP_ProjectailBase_C" (`KismetMathLibrary.MakeTransform` (`KismetMathLibrary.MakeVector` (.x (.location _returnvalue_7)) (.y (.location _returnvalue_7)) (- (.z (.location _returnvalue_7)) 200.0)) (.rotation _returnvalue_7) (.scale _returnvalue_7)) "Undefined" "MultiplyWithRoot" null 600.0 0.0 "/Game/sA_Megapack_v1/sA_Projectilevfx/Vfx/Fx/Niagara_Systems/NS_Hit7.NS_Hit7" null null)
  (`KismetSystemLibrary.Delay` 0.5)
  (`|SpawnActorFromClass` "/Game/Blueprint/Damage/BP_ProjectailBase.BP_ProjectailBase_C" (`KismetMathLibrary.MakeTransform` (`KismetMathLibrary.MakeVector` (.x (.location _returnvalue_8)) (.y (.location _returnvalue_8)) (- (.z (.location _returnvalue_8)) 50.0)) (.rotation _returnvalue_8) (.scale _returnvalue_8)) "Undefined" "MultiplyWithRoot" null 600.0 0.0 "/Game/sA_Megapack_v1/sA_Projectilevfx/Vfx/Fx/Niagara_Systems/NS_Hit7.NS_Hit7" null null)
  (`KismetSystemLibrary.Delay` 0.5)
  (`|SpawnActorFromClass` "/Game/Blueprint/Damage/BP_ProjectailBase.BP_ProjectailBase_C" (`KismetMathLibrary.MakeTransform` (`KismetMathLibrary.MakeVector` (.x (.location _returnvalue_9)) (.y (.location _returnvalue_9)) (+ (.z (.location _returnvalue_9)) 50.0)) (.rotation _returnvalue_9) (.scale _returnvalue_9)) "Undefined" "MultiplyWithRoot" null 1000.0 0.0 "/Game/sA_Megapack_v1/sA_Projectilevfx/Vfx/Fx/Niagara_Systems/NS_Hit7.NS_Hit7" null null)
  (set `self.Attack3?` false))

(event `Attack2`
  (bind _returnvalue (`self.GetTransform`))
  ;[0.15 0.15 0.15 0.5 100] Attack2
  (set `self.Attack2?` true)
  (`GameplayStatics.PlaySound2D` null 1.0 1.0 0.0 null null)
  (bind _returnvalue_2 (`|SpawnActorFromClass` "/Game/Blueprint/Damage/BP_AtackBossFullArea.BP_AtackBossFullArea_C" (`KismetMathLibrary.MakeTransform` (`KismetMathLibrary.MakeVector` (.x (.location _returnvalue)) (.y (.location _returnvalue)) (- (.z (.location _returnvalue)) 250.0)) (.rotation _returnvalue)) "Undefined" "MultiplyWithRoot" null null))
  (`KismetSystemLibrary.Delay` 4.0)
  (`self.K2_DestroyActor` _returnvalue_2)
  (set `self.Attack2?` false))

(event `Attack1`
  ;[0.15 0.15 0.15 0.5 100] Attack1
  (`GameplayStatics.PlaySound2D` null 1.0 1.0 0.0 null null)
  (`KismetSystemLibrary.Delay` 0.2)
  (bind _outlaunchvelocity (`GameplayStatics.SuggestProjectileVelocity_CustomArc` (`self.K2_GetActorLocation`) (60.0 -1.0 20.0)))
  (`self.LaunchCharacter` _outlaunchvelocity true true)
  (`KismetSystemLibrary.Delay` 1.5)
  (bind _outlaunchvelocity_2 (`GameplayStatics.SuggestProjectileVelocity_CustomArc` (`self.K2_GetActorLocation`) (-730.0 -1.0 20.0)))
  (`self.LaunchCharacter` _outlaunchvelocity_2 true true)
  (`KismetSystemLibrary.Delay` 1.5)
  (`SceneComponent.K2_SetRelativeRotation` (`self.Sprite`) (struct :`Yaw` -180.0) false false)
  (`KismetSystemLibrary.Delay` 1.0)
  (bind _outlaunchvelocity_3 (`GameplayStatics.SuggestProjectileVelocity_CustomArc` (`self.K2_GetActorLocation`) (60.0 -1.0 20.0)))
  (`self.LaunchCharacter` _outlaunchvelocity_3 true true)
  (`KismetSystemLibrary.Delay` 1.5)
  (bind _outlaunchvelocity_4 (`GameplayStatics.SuggestProjectileVelocity_CustomArc` (`self.K2_GetActorLocation`) (850.0 -1.0 20.0)))
  (`self.LaunchCharacter` _outlaunchvelocity_4 true true)
  (`KismetSystemLibrary.Delay` 1.5)
  (`SceneComponent.K2_SetRelativeRotation` :`self` (`self.Sprite`)))

(event `self.ReceiveBeginPlay`
  (`self.Attack`))

(event `Attack`
  (if (`self.Dead`)
    _
    (elif (<= (`self.Health`) 500.0)
      (if (<= (`self.Health`) 200.0)
        (switch `int` (`KismetMathLibrary.RandomIntegerInRange` 0 2)
          (:`0`
            (`self.Attack4`)
            (`self.Attack3`)
            (`KismetSystemLibrary.Delay` 12.0)
            (`self.Attack`))
          (:`1`
            (`self.Attack1`)
            (`self.Attack4`)
            (`KismetSystemLibrary.Delay` 10.0)
            (`self.Attack`))
          (:`2`
            (`self.Attack2`)
            (`self.Attack5`)
            (`KismetSystemLibrary.Delay` 10.0)
            (`self.Attack`)))
        (else
          (switch `int` (`KismetMathLibrary.RandomIntegerInRange` 0 4)
            (:`0`
              (`self.Attack1`)
              (`KismetSystemLibrary.Delay` 10.0)
              (`self.Attack`))
            (:`1`
              (`self.Attack2`)
              (`KismetSystemLibrary.Delay` 6.0)
              (`self.Attack`))
            (:`2`
              (`self.Attack3`)
              (`KismetSystemLibrary.Delay` 10.0)
              (`self.Attack`))
            (:`3`
              (`self.Attack4`)
              (`KismetSystemLibrary.Delay` 10.0)
              (`self.Attack`))
            (:`4`
              (`self.Attack5`)
              (`KismetSystemLibrary.Delay` 4.0)
              (`self.Attack`)))))
      (else
        (switch `int` (`KismetMathLibrary.RandomIntegerInRange` 0 2)
          (:`0`
            (`self.Attack1`)
            (`KismetSystemLibrary.Delay` 10.0)
            (`self.Attack`))
          (:`1`
            (`self.Attack2`)
            (`KismetSystemLibrary.Delay` 6.0)
            (`self.Attack`))
          (:`2`
            (`self.Attack3`)
            (`KismetSystemLibrary.Delay` 10.0)
            (`self.Attack`)))))))

(event `self.ReceiveAnyDamage`
  (params (Damage :type "Float (single-precision)") (DamageType :type "DamageType Object Reference") (InstigatedBy :type "Controller Object Reference") (DamageCauser :type "Actor Object Reference"))
  (bind _returnvalue (`self.GetTransform`))
  (if (not (`self.Dead`))
    (set `self.Health` (- (`self.Health`) Damage))
    (if (<= (`self.Health`) 0.0)
      (`PaperZDAnimInstance.JumpToNode` (`PaperZDAnimationComponent.AnimInstance` (`self.AnimationComponent`)) "Dead" "None")
      (set `self.Dead` true)
      (`KismetSystemLibrary.Delay` 2.0)
      (`self.K2_DestroyActor`)
      (`|SpawnActorFromClass` "/Game/Blueprint/BP_Cards.BP_Cards_C" (`KismetMathLibrary.MakeTransform` (`KismetMathLibrary.MakeVector` (.x (.location _returnvalue)) (.y (.location _returnvalue)) -150.0)) "Undefined" "MultiplyWithRoot" null null)
      (else
        (set `self.Hurt?` true)
        (`PaperZDAnimInstance.JumpToNode` (`PaperZDAnimationComponent.AnimInstance` (`self.AnimationComponent`)) "Hurt" "None")
        (`KismetSystemLibrary.Delay` 0.5)
        (set `self.Hurt?` false)))))

(event `self.Box.OnComponentBeginOverlap`
  (params (OverlappedComponent :type "PrimitiveComponent Object Reference") (OtherActor :type "Actor Object Reference") (OtherComp :type "PrimitiveComponent Object Reference") (OtherBodyIndex :type Integer) (bFromSweep :type Boolean) (SweepResult :type "HitResult Structure (by ref)"))
  (bind _asbp_hero (cast `/Game/Blueprint/Hero/BP_Hero` OtherActor))
  (set `self.Char` _asbp_hero)
  (set `self.On?` true))

(event `self.Box.OnComponentEndOverlap`
  (params (OverlappedComponent :type "PrimitiveComponent Object Reference") (OtherActor :type "Actor Object Reference") (OtherComp :type "PrimitiveComponent Object Reference") (OtherBodyIndex :type Integer))
  (cast `/Game/Blueprint/Hero/BP_Hero` OtherActor)
  (set `self.On?` false))

(event `self.ReceiveTick`
  (params (DeltaSeconds :type "Float (single-precision)"))
  (`KismetSystemLibrary.Delay` 1.0)
  (if (`self.On?`)
    (`GameplayStatics.ApplyDamage` (`self.Char`) 1.0)))

(fn `SpawnDust`
  (bind (_returnvalue_location _returnvalue_rotation) (`KismetMathLibrary.BreakTransform` (`SceneComponent.K2_GetComponentToWorld` (`self.Sprite`))))
  (`|SpawnActorFromClass` "/Game/Blueprint/Hero/BP_LandDust.BP_LandDust_C" (`KismetMathLibrary.MakeTransform` _returnvalue_location _returnvalue_rotation) "Undefined" "MultiplyWithRoot" null null))

(fn `UserConstructionScript`)